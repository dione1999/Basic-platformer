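; Key pickup item that grants a key to the player character when picked up.
; It extends a parent pickup class, running the inherited PickUpEvent logic before its own.
; It then casts the pickup owner to GG_Char_BP and passes its KeyTypeTag to GetKeyFunction, so the tag identifies which key is given.
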(event EventBeginPlay
  (|CallParentFunction) ; This node is disabled and will not be called.\nDrag off pins to build functionality.
)

(event Collision|EventActorBeginOverlap
  (params (OtherActor :type Actor%20Object%20Reference))
  (|CallParentFunction OtherActor) ; This node is disabled and will not be called.\nDrag off pins to build functionality.
)

(event EventTick
  (params (DeltaSeconds :type Float%20%28single-precision%29))
  (|CallParentFunction DeltaSeconds) ; This node is disabled and will not be called.\nDrag off pins to build functionality.
)

(event EventPickUpEvent
  (params (actor%20-%20pick%20up%20owner%20 :type Actor%20Object%20Reference))
  ;[1 1 1] play sound
  (|CallParentFunction actor%20-%20pick%20up%20owner%20)
  ;[1 1 1] key checking
  (bind _asgg_char_bp (Utilities|Casting|CastToGG_Char_BP actor%20-%20pick%20up%20owner%20))
  (Default|GetKey(function) _asgg_char_bp (Variables|Default|GetKeyType_Tag)))

(fn ConstructionScript
  (|CallParentFunction))