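; Checkpoint barrier actor that acts as a force field, opening only once the blue key has been obtained.
; BeginPlay creates a dynamic material instance on the Barior component.
; EventCheckPoint checks GotKey: if set, a timeline fades the material's Opacity, collision is disabled and the actor is destroyed after a delay.
; Without the key, it prints a hint to get the blue key.
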(event EventBeginPlay
  (|CallParentFunction)
  ;[1 1 1] matrial fading anim
  (bind _returnvalue (Rendering|Material|CreateDynamicMaterialInstance (Variables|Default|Getbarior) 0 (Variables|Default|GetSource%20Material) "None" :!class /Script/Engine.PrimitiveComponent))
  (Variables|Default|SetSlow%20Fading%20Anim _returnvalue))

(event Collision|EventActorBeginOverlap
  (params (OtherActor :type Actor%20Object%20Reference))
  (|CallParentFunction OtherActor) ; This node is disabled and will not be called.\nDrag off pins to build functionality.
)

(event EventTick
  (params (DeltaSeconds :type Float%20%28single-precision%29))
  (|CallParentFunction DeltaSeconds) ; This node is disabled and will not be called.\nDrag off pins to build functionality.
)

(event EventCheckPoint(E)
  (if (Variables|Default|GetGot%20key)
    ;[1 1 1] force field fading anim
    (bind _opacity (Timeline|Matiral%20Fading%20Timeline Play)
      (:Update
        (Rendering|Material|SetScalarParameterValue (Variables|Default|GetSlow%20Fading%20Anim) "Opacity" _opacity :!class /Script/Engine.MaterialInstanceDynamic)
        (Collision|SetCollisionEnabled (Variables|Default|Getbarior) "NoCollision")
        (Utilities|FlowControl|Delay 4.0)
        (Actor|DestroyActor)))
    (else
      (Development|PrintString "get blue key"))))

(fn ConstructionScript
  (|CallParentFunction))